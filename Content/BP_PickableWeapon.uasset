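; BP_PickableWeapon is a world weapon pickup that a first-person character can collect.
; Its construction script applies the mesh and name from GunStats to the weapon component and text label, and passes those stats on as the weapon's GunConfig.
; On pickup, TPWeapon attaches to the character, and on success the first-person arms AnimBP's HasRifle flag is set to switch to rifle animations.
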(event `self.TP_PickUp.OnPickUp`
  (params (PickUpCharacter :type "DataDrivenFPTCharacter Object Reference"))
  (bind _returnvalue (`TP_WeaponComponent.AttachWeapon` (`self.TP_Weapon`) PickUpCharacter))
  (if _returnvalue
    (bind _asfirst_person_anim_bp (cast `/Game/FirstPersonArms/Animations/FirstPerson_AnimBP` (`SkeletalMeshComponent.GetAnimInstance` (`DataDrivenFPTCharacter.Mesh1P` PickUpCharacter))))
    (set `/Game/FirstPersonArms/Animations/FirstPerson_AnimBP.HasRifle` true _asfirst_person_anim_bp)))

(fn `UserConstructionScript`
  (bind _gunstats (`self.GunStats`))
  (`SkeletalMeshComponent.SetSkeletalMeshAsset` (`self.TP_Weapon`) (`DA_GunStats.GunMesh` _gunstats))
  (`TextRenderComponent.K2_SetText` (`self.TextRender`) (`KismetTextLibrary.Conv_StringToText` (`DA_GunStats.GunName` _gunstats)))
  (set `TP_WeaponComponent.GunConfig` (`self.GunStats`) (`self.TP_Weapon`)))